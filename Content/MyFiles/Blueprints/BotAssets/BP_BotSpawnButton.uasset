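; Interactable button that toggles target bot spawning for a first-person shooting activity.
; A box overlap enables input while the player is in range and adds the score UI to the viewport on first entry.
; Interact alternates through a FlipFlop between a delayed, flag-guarded SpawnBot call on the referenced spawner, and resetting the score before destroying all BP_BotToShoot actors.
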(event OnComponentBeginOverlap(Box)
  (params (OverlappedComponent :type Primitive%20Component%20Object%20Reference) (OtherActor :type Actor%20Object%20Reference) (OtherComp :type Primitive%20Component%20Object%20Reference) (OtherBodyIndex :type Integer) (bFromSweep :type Boolean) (SweepResult :type Hit%20Result%20Structure%20%28by%20ref%29))
  (bind _asbp_first_person_character (Utilities|Casting|CastToBP_FirstPersonCharacter OtherActor))
  (Input|EnableInput (Game|GetPlayerController 0)) ; Allow player to press "E"
  ;[1 1 1] Adds Score UI when user stands in front of button
  (Utilities|FlowControl|DoOnce false
    (:Completed
      (UserInterface|Viewport|AddtoViewport (Variables|/Game/FirstPerson/Blueprints/BP_FirstPersonCharacter.BP_FirstPersonCharacter_C|GetUI _asbp_first_person_character) 0))))

(event OnComponentEndOverlap(Box)
  (params (OverlappedComponent :type Primitive%20Component%20Object%20Reference) (OtherActor :type Actor%20Object%20Reference) (OtherComp :type Primitive%20Component%20Object%20Reference) (OtherBodyIndex :type Integer))
  (Utilities|Casting|CastToBP_FirstPersonCharacter OtherActor)
  (Input|DisableInput (Game|GetPlayerController 0)))

(event Input|ActionEvents|InputActionInteract
  (params (Key :type Key%20Structure :default "None"))
  (:Pressed
    (Utilities|FlowControl|FlipFlop ; Toggle Interact on Bot Spawn Button
      (:A
        ;[1 1 1] Starting Bot Spawn
        (Audio|PlaySoundatLocation "/Game/MyFiles/SFX/button_press.button_press" (Transformation|GetWorldLocation (Variables|/Game/FirstPerson/Blueprints/BP_FirstPersonCharacter.BP_FirstPersonCharacter_C|GetFirstPersonCamera (stale OnComponentBeginOverlap(Box) _asbp_first_person_character))) "0, 0, 0" 1.0 1.0 0.0 0 0 0 0)
        (if (not (Variables|Default|GethasAlreadySpawned?))
          (Variables|Default|SethasAlreadySpawned? true)
          (Utilities|FlowControl|Delay 1.5)
          (Default|SpawnBot (Variables|Default|Getbotspawnerref))))
      (:B
        ;[1 1 1] Score update when turning off bots
        (Audio|PlaySoundatLocation "/Game/MyFiles/SFX/button_press.button_press" (Transformation|GetWorldLocation (Variables|/Game/FirstPerson/Blueprints/BP_FirstPersonCharacter.BP_FirstPersonCharacter_C|GetFirstPersonCamera (stale OnComponentBeginOverlap(Box) _asbp_first_person_character))) "0, 0, 0" 1.0 1.0 0.0 0 0 0 0)
        (Variables|/Game/FirstPerson/Blueprints/BP_FirstPersonCharacter.BP_FirstPersonCharacter_C|SetplayerScore (stale OnComponentBeginOverlap(Box) _asbp_first_person_character) 0)
        (Rendering|Components|TextRender|SetText (Variables|/Game/MyFiles/Blueprints/UI/UI_botScore.UI_botScore_C|GetScoreValue (Variables|/Game/FirstPerson/Blueprints/BP_FirstPersonCharacter.BP_FirstPersonCharacter_C|GetUI (stale OnComponentBeginOverlap(Box) _asbp_first_person_character))) (Utilities|Text|ToText(Integer) (Variables|Default|GetresetScore)))
        (Utilities|FlowControl|Delay 0.4)
        (bind _outactors (Actor|GetAllActorsOfClass "/Game/MyFiles/Blueprints/BotAssets/BP_BotToShoot.BP_BotToShoot_C"))
        (Variables|Default|SethasAlreadySpawned? false)
        (Actor|DestroyActor _outactors)))))

(fn ConstructionScript)