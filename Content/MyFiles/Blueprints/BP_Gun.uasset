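; BP_Gun is a gun pickup that gives the first-person character its weapon mesh.
; The construction script shows the Gun skeletal mesh on GunMesh.
; When the character overlaps Box, the actor enables player input, and pressing E then copies that mesh onto the character's FPGun component.
; Nothing in the graph disables input again or removes the pickup.
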(event OnComponentBeginOverlap(Box)
  (params (OverlappedComponent :type Primitive%20Component%20Object%20Reference) (OtherActor :type Actor%20Object%20Reference) (OtherComp :type Primitive%20Component%20Object%20Reference) (OtherBodyIndex :type Integer) (bFromSweep :type Boolean) (SweepResult :type Hit%20Result%20Structure%20%28by%20ref%29))
  ;[1 1 1] Simple gun pickup
  (Utilities|Casting|CastToBP_FirstPersonCharacter OtherActor)
  (Input|EnableInput (Game|GetPlayerController 0)))

(event Input|KeyboardEvents|E
  (params (Key :type Key%20Structure :default "None"))
  ;[1 1 1] pick up gun with keyboard input
  (:Pressed
    (bind _asbp_first_person_character (Utilities|Casting|CastToBP_FirstPersonCharacter (Game|GetPlayerCharacter 0)))
    (Class|SkinnedMeshComponent|SetSkeletalMesh (Variables|/Game/FirstPerson/Blueprints/BP_FirstPersonCharacter.BP_FirstPersonCharacter_C|GetFPGun _asbp_first_person_character) (Variables|Default|GetGun) true)))

(fn ConstructionScript
  (Class|SkinnedMeshComponent|SetSkeletalMesh (Variables|Default|GetGun%20Mesh) (Variables|Default|GetGun) true))