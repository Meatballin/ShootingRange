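; BP_BotSpawner keeps one BP_BotToShoot target bot in the level, respawning it whenever it is destroyed.
; On BeginPlay it spawns a bot at the world location of a randomly chosen one of its eleven Arrow components, with a fixed rotation.
; It binds to each bot's OnDestroyed event, which calls SpawnBot again to place the replacement at a new random point.
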(event Custom|Spawn%20Bot
  (bind _returnvalue (Game|SpawnActorfromClass "/Game/MyFiles/Blueprints/BP_BotToShoot.BP_BotToShoot_C" (Math|Transform|MakeTransform (Transformation|GetWorldLocation (Utilities|Array|Get(acopy) (Utilities|Array|MakeArray (Variables|Default|GetArrow) (Variables|Default|GetArrow1) (Variables|Default|GetArrow2) (Variables|Default|GetArrow3) (Variables|Default|GetArrow4) (Variables|Default|GetArrow5) (Variables|Default|GetArrow6) (Variables|Default|GetArrow7) (Variables|Default|GetArrow8) (Variables|Default|GetArrow9) (Variables|Default|GetArrow10)) (Math|Random|RandomIntegerinRange 0 10))) "0,180.000000, 0") "Undefined" 0 0))
  (Game|AssignOnDestroyed _returnvalue (delegate Custom|NeedToRespawn)))

(event Custom|NeedToRespawn
  (params (DestroyedActor :type Actor%20Object%20Reference))
  (CallFunction|SpawnBot))

(event EventBeginPlay
  (CallFunction|SpawnBot))

(fn ConstructionScript)