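; Interactable button that starts and stops the bot shooting session.
; Overlapping its box as the first-person character caches that character and enables input, with no end-overlap to disable it.
; Interact alternates through a FlipFlop: one press calls SpawnBot on the referenced spawner after a short delay, guarded by a flag.
; The next press zeroes the player's score, updates the UI, destroys all BP_BotToShoot actors and clears the flag.
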(event OnComponentBeginOverlap(Box)
  (params (OverlappedComponent :type Primitive%20Component%20Object%20Reference) (OtherActor :type Actor%20Object%20Reference) (OtherComp :type Primitive%20Component%20Object%20Reference) (OtherBodyIndex :type Integer) (bFromSweep :type Boolean) (SweepResult :type Hit%20Result%20Structure%20%28by%20ref%29))
  (bind _asbp_first_person_character (Utilities|Casting|CastToBP_FirstPersonCharacter OtherActor))
  (Input|EnableInput (Game|GetPlayerController 0)) ; Allow player to press "E"
)

(event Input|ActionEvents|InputActionInteract
  (params (Key :type Key%20Structure :default "None"))
  (:Pressed
    (Utilities|FlowControl|FlipFlop ; Toggle Interact on Bot Spawn Button
      (:A
        ;[1 1 1] Starting Bot Spawn
        (if (not (Variables|Default|GethasAlreadySpawned?))
          (Variables|Default|SethasAlreadySpawned? true)
          (Utilities|FlowControl|Delay 1.5)
          (Default|SpawnBot (Variables|Default|Getbotspawnerref))))
      (:B
        ;[1 1 1] Score update when turning off bots
        (Variables|/Game/FirstPerson/Blueprints/BP_FirstPersonCharacter.BP_FirstPersonCharacter_C|SetplayerScore (stale OnComponentBeginOverlap(Box) _asbp_first_person_character) 0)
        (Rendering|Components|TextRender|SetText (Variables|/Game/MyFiles/Blueprints/UI_botScore.UI_botScore_C|GetScoreValue (Variables|/Game/FirstPerson/Blueprints/BP_FirstPersonCharacter.BP_FirstPersonCharacter_C|GetUI (stale OnComponentBeginOverlap(Box) _asbp_first_person_character))) (Utilities|Text|ToText(Integer) (Variables|Default|GetresetScore)))
        (bind _outactors (Actor|GetAllActorsOfClass "/Game/MyFiles/Blueprints/BP_BotToShoot.BP_BotToShoot_C"))
        (Variables|Default|SethasAlreadySpawned? false)
        (Actor|DestroyActor _outactors)))))

(fn ConstructionScript)